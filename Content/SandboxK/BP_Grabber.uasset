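; Grabber component that lets the player pick up, carry and drop an actor with the F key.
; F sphere-traces a short distance along the component's forward vector to store the hit actor and component, or flags a release when already holding.
; Tick pins the held actor to the trace end point with physics simulation off on the hit component, then re-enables physics and clears the references on release.
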(event EventBeginPlay
  ;[1 1 1] Set Defalut Value
  (Variables|Default|SetGrabbingDistance 1.3e+02)
  (Variables|Default|SetHaveItem false)
  (Variables|Default|SetWannaRelase false))

(event EventTick
  (params (DeltaSeconds :type Float%20%28single-precision%29))
  ;[1 1 1] Update Start & End Location Var
  (bind _output_get (Variables|Default|SetStart (Transformation|GetWorldLocation)))
  (Variables|Default|SetEnd (+ _output_get (* (Math|Vector|GetForwardVector) (Variables|Default|GetGrabbingDistance))))
  ;[1 1 1] If (HaveItem && !WannaRelase)
  (if (Utilities|IsValid (Variables|Default|GetGrabbedActor))
    (bind _output_get_2 (Variables|Default|SetHaveItem true))
    (if (and _output_get_2 (not (Variables|Default|GetWannaRelase)))
      ;[1 1 1] Move Grabbed Actor
      (Transformation|SetActorLocationAndRotation (Variables|Default|GetGrabbedActor) (Variables|Default|GetEnd))
      (if (Utilities|IsValid (Variables|Default|GetGrabbedItem))
        (Physics|SetSimulatePhysics (Variables|Default|GetGrabbedItem) false))
      (else
        ;[1 1 1] Relase Grabbed Actor
        (if (Variables|Default|GetHaveItem)
          (Physics|SetSimulatePhysics (Variables|Default|GetGrabbedItem) true)
          (Variables|Default|SetGrabbedActor 0)
          (Variables|Default|SetGrabbedItem 0)
          (Variables|Default|SetHaveItem false)
          (Variables|Default|SetWannaRelase false))))
    (else
      (Variables|Default|SetHaveItem false))))

(event Input|KeyboardEvents|F
  (params (Key :type Key%20Structure :default "None"))
  ;[1 1 1] Press "F" To Find OR Relase Actor
  (:Pressed
    (if (Variables|Default|GetHaveItem)
      (Variables|Default|SetWannaRelase true)
      (else
        (bind (_outhit _returnvalue) (Collision|SphereTraceByChannel (Variables|Default|GetStart) (Variables|Default|GetEnd) 4e+01 "TraceTypeQuery3" false 0 "None"))
        (if _returnvalue
          (Variables|Default|SetHaveItem true)
          (Variables|Default|SetGrabbedActor (.HitActor (Collision|BreakHitResult _outhit)))
          (Variables|Default|SetGrabbedItem (.HitComponent (Collision|BreakHitResult _outhit))))))))