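; BP_Crafted is an item Blueprint for crafted objects, identified by a "Crafted" tag.
; Its construction script adds that tag, then loops through the recipe data table's row names to fetch the row matching its ID.
; The assignments of Name, Points and TimeToCraft from that row are disconnected, so the lookup currently stores nothing.
; BeginPlay only calls the parent.
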(event EventBeginPlay
  (|CallParentFunction))

(event Collision|EventActorBeginOverlap
  (params (OtherActor :type Actor%20Object%20Reference)))

(event EventTick
  (params (DeltaSeconds :type Float%20%28single-precision%29)))

(fn ConstructionScript
  (bind _recipe_datatable (Variables|Default|GetRecipe%20DataTable))
  (|CallParentFunction)
  ;[0.09306 0.09306 0.09306] Tag Setup
  (Utilities|Array|AddUnique (Variables|Default|GetTags) "Crafted")
  (bind _outrownames (DataTable|GetDataTableRowNames _recipe_datatable))
  (for _array_element _outrownames
    (if (== _array_element (Variables|Default|GetID))
      (bind _returnvalue (Utilities|GetDataTableRow _recipe_datatable _array_element)))))