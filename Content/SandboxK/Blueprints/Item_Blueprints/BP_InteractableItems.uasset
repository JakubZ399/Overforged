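; BP_InteractableItems is an interactable item actor with a mesh and a 2D widget image meant to display over the object.
; MeshToRootSetup assigns a given mesh to CoreMesh, and SetupDisplayImage passes the item's image and desired size to the W_Flower widget in Image2D.
; Both helper calls are disconnected in this Blueprint, so BeginPlay and the construction script do nothing here.
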(event EventBeginPlay)

(fn ConstructionScript)

(fn MeshtoRootSetup
  (params (MeshToRoot :type Static%20Mesh%20Object%20Reference))
  (Components|StaticMesh|SetStaticMesh (Variables|Default|GetCoreMesh) MeshToRoot))

(fn SetupDisplayImage
  (bind _asw_flower (Utilities|Casting|CastToW_Flower (UserInterface|GetWidget (Variables|Default|GetImage2D))))
  ;[1 1 1] Setup Display Image Over Object
  (Utilities|FlowControl|Sequence
    (:then_0
      (Variables|/Game/SandboxK/UI/W_Flower.W_Flower_C|SetPopUpSlateBrush _asw_flower (Variables|Default|GetItemImage)))
    (:then_1
      (Variables|/Game/SandboxK/UI/W_Flower.W_Flower_C|SetImage%20Size%20X _asw_flower (Variables|ImageSize|GetDesired%20Size%20X)))
    (:then_2
      (Variables|/Game/SandboxK/UI/W_Flower.W_Flower_C|SetImage%20Size%20Y _asw_flower (Variables|ImageSize|GetDesired%20Size%20Y)))))