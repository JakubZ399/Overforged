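; BP_StorageBox is a flower storage box that spawns one type of flower, chosen per instance through ItemList.
; The construction script sets the box's top material and the flower class to spawn from that selection.
; ItemTrigger overlaps toggle HavePlace, marking the spot occupied on begin and free on end.
; AddItem spawns the flower at a fixed height above the box collision, only while HavePlace is true.
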(event OnComponentBeginOverlap(ItemTrigger)
  (params (OverlappedComponent :type Primitive%20Component%20Object%20Reference) (OtherActor :type Actor%20Object%20Reference) (OtherComp :type Primitive%20Component%20Object%20Reference) (OtherBodyIndex :type Integer) (bFromSweep :type Boolean) (SweepResult :type Hit%20Result%20Structure%20%28by%20ref%29))
  (Variables|Default|SetHavePlace false))

(event OnComponentEndOverlap(ItemTrigger)
  (params (OverlappedComponent :type Primitive%20Component%20Object%20Reference) (OtherActor :type Actor%20Object%20Reference) (OtherComp :type Primitive%20Component%20Object%20Reference) (OtherBodyIndex :type Integer))
  (Variables|Default|SetHavePlace true))

(fn ConstructionScript
  (bind _boxupmesh (Variables|Default|GetBoxUpMesh))
  (switch Utilities|FlowControl|Switch|SwitchonE_Ingredient (Variables|Default|GetItemList)
    (:NewEnumerator0
      (Rendering|Material|SetMaterial _boxupmesh 0 "/Game/R_Models/Box/Box/MI_Box_Daff.MI_Box_Daff")
      (Variables|Default|SetItemToTake "/Game/SandboxK/Blueprints/Interactable_Items/BP_Flower_Daff.BP_Flower_Daff_C"))
    (:NewEnumerator1
      (Rendering|Material|SetMaterial _boxupmesh 0 "/Game/R_Models/Box/Box/MI_Box_Lily.MI_Box_Lily")
      (Variables|Default|SetItemToTake "/Game/SandboxK/Blueprints/Interactable_Items/BP_Flower_Lily.BP_Flower_Lily_C"))
    (:NewEnumerator2
      (Rendering|Material|SetMaterial _boxupmesh 0 "/Game/R_Models/Box/Box/MI_Box_Ribbon.MI_Box_Ribbon")
      (Variables|Default|SetItemToTake "/Game/SandboxK/Blueprints/Interactable_Items/BP_Flower_Ribbon.BP_Flower_Ribbon_C"))
    (:NewEnumerator3
      (Rendering|Material|SetMaterial _boxupmesh 0 "/Game/R_Models/Box/Box/MI_BoxDaisy.MI_BoxDaisy")
      (Variables|Default|SetItemToTake "/Game/SandboxK/Blueprints/Interactable_Items/BP_Flower_Daisy.BP_Flower_Daisy_C"))
    (:NewEnumerator4
      (Rendering|Material|SetMaterial _boxupmesh 0 "/Game/R_Models/Box/Box/MI_BoxRose.MI_BoxRose")
      (Variables|Default|SetItemToTake "/Game/SandboxK/Blueprints/Interactable_Items/BP_Flower_Rose.BP_Flower_Rose_C"))))

(fn AddItem
  (bind _storageboxcollision (Variables|Default|GetStorageBoxCollision))
  (bind _returnvalue (Transformation|GetWorldLocation _storageboxcollision))
  (bind (_x _y _z) (Math|Vector|BreakVector _returnvalue))
  (if (Variables|Default|GetHavePlace)
    (Game|SpawnActorfromClass (Variables|Default|GetItemToTake) (Math|Conversions|ToTransform(Vector) (Math|Vector|MakeVector _x _y (+ _z 1.6e+02))) "Undefined" "MultiplyWithRoot" 0 0)
    (return)))