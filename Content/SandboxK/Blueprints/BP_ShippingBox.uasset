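; BP_ShippingBox is a delivery point that accepts placed items tagged "Crafted" and scores them against active orders.
; PlaceItemInterface hands the item to MoveActor, which glides it onto the box and searches the Order Manager's ActiveOrder for its class.
; On a match, it animates and destroys the item, adds its crafted points to the GameMode score, and removes the order and its UI panel entry.
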(event Custom|MoveActor
  (bind _item (Variables|Default|GetItem))
  (bind _item_2 (Variables|Default|GetItem))
  ;[1 1 1] Move Actor To
  (Transformation|AttachComponentToComponent _item_2 (Variables|Default|GetItemGO) "None" "KeepWorld" "KeepWorld" "KeepWorld" true)
  (Components|MoveComponentTo (Variables|/Script/Engine.Actor|GetRootComponent _item_2) "0, 0, 0" "0, 0, 0" true false 0.2 false)
  ;[1 1 1] Setup Reference To Object
  (bind _asbp_level_game_mode (Utilities|Casting|CastToBP_LevelGameMode (Game|GetGameMode)))
  (bind _asw_level_ui (Utilities|Casting|CastToW_LevelUI (Variables|/Game/SandboxK/Blueprints/BP_LevelGameMode.BP_LevelGameMode_C|GetLevelUI _asbp_level_game_mode)))
  (Variables|Default|SetLevelUI%20Ref _asw_level_ui)
  (bind _output_get (Variables|Default|SetOrderManager%20Ref (Variables|/Game/SandboxK/Blueprints/BP_LevelGameMode.BP_LevelGameMode_C|GetBP_OrderManagerGM _asbp_level_game_mode)))
  ;[1 1 1] Searching For Same Item In Array
  (bind (_array_element _array_index) (Utilities|Array|ForEachLoopwithBreak (Variables|/Game/SandboxK/Blueprints/BP_OrderManager.BP_OrderManager_C|GetActiveOrder _output_get) :!label _label)
    (:LoopBody
      (if (== (.BP (Utilities|Struct|BreakS_OrderStruck _array_element)) (Utilities|GetClass (Variables|Default|GetItem)))
        ;[1 1 1] Add Points & Rotation Animation & Destroy Actor
        (bind _points (Class|BPIItemInterface|GetCraftedPoints(Message) _item))
        (Variables|Default|SetScoreAdd _points)
        (Utilities|FlowControl|Delay (Variables|Default|GetTimeToAddScore))
        (Components|MoveComponentTo (Variables|/Script/Engine.Actor|GetRootComponent _item) "0.000000,0.000000,100.000000" "0.000000,180.000000,0.000000" false true 1.0 false)
        (Actor|DestroyActor _item)
        (bind _asbp_level_game_mode_2 (Utilities|Casting|CastToBP_LevelGameMode (Game|GetGameMode)))
        (Variables|/Game/SandboxK/Blueprints/BP_LevelGameMode.BP_LevelGameMode_C|SetScore _asbp_level_game_mode_2 (+ (Variables|/Game/SandboxK/Blueprints/BP_LevelGameMode.BP_LevelGameMode_C|GetScore _asbp_level_game_mode_2) (Variables|Default|GetScoreAdd)))
        ;[1 1 1] Remove OrderUI From Level_UI & Remove Order From ActiveOrderArray (from OrderManager)
        (bind (_array_element_2 _array_index_2) (Utilities|Array|ForEachLoopwithBreak (Variables|/Game/SandboxK/UI/W_LevelUI.W_LevelUI_C|GetOrderPanelActive (Variables|Default|GetLevelUI%20Ref)) :!label _label_2)
          (:LoopBody
            (bind _asw_order_ui (Utilities|Casting|CastToW_OrderUI _array_element_2))
            (if (== (Variables|/Game/SandboxK/UI/W_OrderUI.W_OrderUI_C|GetOrderNameFromOM _asw_order_ui) (.OrderName (Utilities|Struct|BreakS_OrderStruck _array_element)))
              (bind _returnvalue (Class|PanelWidget|RemoveChildat (Variables|/Game/SandboxK/UI/W_LevelUI.W_LevelUI_C|GetOrderPanelHorizontal (Variables|Default|GetLevelUI%20Ref)) _array_index_2))
              (if _returnvalue
                (Utilities|Array|RemoveIndex (Variables|/Game/SandboxK/Blueprints/BP_OrderManager.BP_OrderManager_C|GetActiveOrder _output_get) _array_index)
                (goto _label_2 Break))))
          (:Completed
            (goto _label Break)))))))

(event Custom|PlaceItemInterface_1_2
  (params (ItemToPlace :type Actor%20Object%20Reference)))

(fn ConstructionScript)

(fn PlaceItemInterface
  (params (ItemToPlace :type Actor%20Object%20Reference))
  (if (Actor|ActorHasTag ItemToPlace "Crafted")
    (bind _output_get (Variables|Default|SetItem ItemToPlace))
    (Transformation|DetachFromActor _output_get "KeepWorld" "KeepWorld" "KeepWorld")
    (CallFunction|MoveActor)
    (return true)))