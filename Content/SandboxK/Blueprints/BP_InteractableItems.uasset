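; BP_InteractableItems is an interactable item actor with a configurable mesh, pop-up image and ingredient category.
; The construction script applies the chosen mesh to CoreMesh.
; On BeginPlay it casts the Image2D component's widget to W_Flower and passes it the image and desired size for display over the object.
; GetIngredientEnum exposes the item's ingredient category.
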(event EventBeginPlay
  (bind _asw_flower (Utilities|Casting|CastToW_Flower (UserInterface|GetWidget (Variables|Default|GetImage2D))))
  ;[1 1 1] Setup Display Image Over Object
  (Utilities|FlowControl|Sequence
    (:then_0
      (Variables|/Game/SandboxK/UI/W_Flower.W_Flower_C|SetPopUpSlateBrush _asw_flower (Variables|Default|GetImage)))
    (:then_1
      (Variables|/Game/SandboxK/UI/W_Flower.W_Flower_C|SetImage%20Size%20X _asw_flower (Variables|Image|GetDesired%20Size%20X)))
    (:then_2
      (Variables|/Game/SandboxK/UI/W_Flower.W_Flower_C|SetImage%20Size%20Y _asw_flower (Variables|Image|GetDesired%20Size%20Y)))))

(fn ConstructionScript
  ;[0.09306 0.09306 0.09306] Mesh Setup
  (Components|StaticMesh|SetStaticMesh (Variables|Default|GetCoreMesh) (Variables|Default|GetMesh)))

(fn GetIngredientEnum
  (return (Variables|Default|GetIngredientCategory)))