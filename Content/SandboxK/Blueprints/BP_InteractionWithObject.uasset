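; Scene component that lets its owner highlight, grab, carry, drop and place objects with the F key.
; Each tick it line-traces forward, puts an overlay material on the hit actor's meshes and moves any held actor to the trace end.
; F grabs via sphere trace or releases, placing items on BPI_TableInteraction actors or calling AddItemMessage on StorageBox-tagged actors when empty-handed.
; Disconnected older placement, physics re-enable and attach-based carry logic remains.
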(event EventTick
  (params (DeltaSeconds :type Float%20%28single-precision%29))
  (bind _end (Variables|Default|GetEnd))
  (bind (_x _y _z) (Math|Vector|BreakVector _end))
  ;[1 1 1] Update Start & End Location Var
  (CallFunction|CalculatePositionVector)
  ;[1 1 1] HighLight
  (bind (_outhit _returnvalue) (Collision|LineTraceByChannel (Variables|Default|GetStart) (Variables|Default|GetEnd) "TraceTypeQuery4" false 0 "None"))
  (bind _output_get (Variables|Default|SetHasDetectEnv _returnvalue))
  (CallFunction|ChangeHighlight _output_get (.HitActor (Collision|BreakHitResult _outhit)))
  ;[0.6719 0.6719 0.6719] GrabItem
  ;;[1 1 1] If (HaveItem && !WannaRelase)
  (if (Utilities|IsValid (Variables|Default|GetGrabbedActor))
    (bind _output_get_2 (Variables|Default|SetHaveItem true))
    (if (and _output_get_2 (not (Variables|Default|GetWannaRelase)))
      ;;[1 1 1] Move Grabbed Actor
      (Transformation|SetActorLocationAndRotation (Variables|Default|GetGrabbedActor) (Math|Vector|MakeVector _x _y (+ _z (Variables|Default|GetGrabbingHeight))))
      (if (Utilities|IsValid (Variables|Default|GetGrabbedItem))
        (Physics|SetSimulatePhysics (Variables|Default|GetGrabbedItem) false))
      (else
        ;;[1 1 1] Relase Grabbed Actor
        (if (Variables|Default|GetHaveItem)
          (Variables|Default|SetGrabbedActor 0)
          (Variables|Default|SetGrabbedItem 0)
          (Variables|Default|SetHaveItem false)
          (Variables|Default|SetWannaRelase false))))
    (else
      (Variables|Default|SetHaveItem false))))

(event EventBeginPlay
  (Variables|Default|SetHand (Components|GetChildComponent self 0)))

(event Input|KeyboardEvents|F
  (params (Key :type Key%20Structure :default "None"))
  (bind _currenthitactor (Variables|Default|GetCurrentHitActor))
  (bind _currenthitactor_2 (Variables|Default|GetCurrentHitActor))
  (bind _grabbedactor (Variables|Default|GetGrabbedActor))
  (:Pressed
    (bind _bool (CallFunction|Find&Relase (Variables|Default|GetHaveItem))) ; Find&Relase
    (if _bool
      (Utilities|IsValid _currenthitactor_2
        (:Is%20Valid
          (if (and (Utilities|DoesObjectImplementInterface _currenthitactor_2 "/Game/SandboxK/BPI_TableInteraction.BPI_TableInteraction_C") (Variables|Default|GetHaveItem))
            ;[1 1 1] Place Item On Table Object
            (Utilities|IsValid _grabbedactor
              (:Is%20Valid
                (bind _newparam (Class|BPITableInteraction|PlaceItemInterface(Message) (Variables|Default|GetCurrentHitActor) _grabbedactor))
                (if _newparam
                  (Variables|Default|SetWannaRelase true)
                  (Variables|Default|SetHaveItem false))))
            (else
              ;[1 1 1] Take Item From BP_StorageBox
              (if (and (Actor|ActorHasTag _currenthitactor "StorageBox") (not (Variables|Default|GetHaveItem)))
                (Class|BPIStorageInteraction|AddItem(Message) _currenthitactor)))))))))

(event Input|KeyboardEvents|G
  (params (Key :type Key%20Structure :default "None")))

(fn CalculatePositionVector
  (bind _output_get (Variables|Default|SetStart (Transformation|GetWorldLocation)))
  (Variables|Default|SetEnd (+ _output_get (* (Math|Vector|GetForwardVector) (Variables|Default|GetGrabbingDistance))))
  (return))

(fn ChangeHighlight
  (params (Condition :type Boolean) (CurrentHitActor :type Actor%20Object%20Reference))
  (if Condition ; Detect Hit
    ;[1 1 1] Set HighLight Material
    (bind _output_get (Variables|Default|SetCurrentHitActor CurrentHitActor))
    (bind _array_element (Utilities|Array|ForEachLoopwithBreak (Actor|GetComponentsByClass _output_get "/Script/Engine.MeshComponent"))
      (:LoopBody
        (Rendering|Material|SetOverlayMaterial _array_element "/Game/SandboxK/Materials/M_HighLightPROTOTYPE.M_HighLightPROTOTYPE" :!class /Script/Engine.MeshComponent))
      (:Completed
        ;[1 1 1] Set LastHitActor Material To NONE
        (if (and (!= _output_get (Variables|Default|GetLastHitActor)) (!= (Variables|Default|GetLastHitActor) 0))
          (bind _array_element_2 (Utilities|Array|ForEachLoopwithBreak (Actor|GetComponentsByClass (Variables|Default|GetLastHitActor) "/Script/Engine.MeshComponent") :!label _label)
            (:LoopBody
              (Rendering|Material|SetOverlayMaterial _array_element_2 0 :!class /Script/Engine.MeshComponent))
            (:Completed
              (Variables|Default|SetLastHitActor (Variables|Default|GetCurrentHitActor) :!label _label_2)
              (return)))
          (else
            (goto _label_2)))))
    (else
      ;[1 0 0.03182] If You Change Look You Change Overlay to NONE
      (if (!= (Variables|Default|GetLastHitActor) 0)
        (goto _label)))))

(fn Find&Relase
  (params (Condition :type Boolean))
  (bind _start (Variables|Default|GetStart))
  (bind _end (Variables|Default|GetEnd))
  (bind (_x _y _z) (Math|Vector|BreakVector _start))
  (bind (_x_2 _y_2 _z_2) (Math|Vector|BreakVector _end))
  (if Condition
    (if (Utilities|DoesObjectImplementInterface (Variables|Default|GetCurrentHitActor) "/Game/SandboxK/BPI_TableInteraction.BPI_TableInteraction_C")
      (return true)
      (else
        (Variables|Default|SetWannaRelase true)))
    (else
      (bind (_outhit _returnvalue) (Collision|SphereTraceByChannel (Math|Vector|MakeVector _x _y (+ _z 5e+01)) (Math|Vector|MakeVector _x_2 _y_2 (+ _z_2 5e+01)) 5e+01 "TraceTypeQuery3" false 0 "None"))
      (if _returnvalue
        (Variables|Default|SetHaveItem true)
        (Variables|Default|SetGrabbedActor (.HitActor (Collision|BreakHitResult _outhit)))
        (Variables|Default|SetGrabbedItem (.HitComponent (Collision|BreakHitResult _outhit)))
        (else
          (return true)))))
  (return false))