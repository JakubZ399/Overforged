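; Crafting station actor that turns two "Ingredient"-tagged actors into a spawned BP_Bouquet.
; Overlapping ingredients are destroyed and counted, filling a circular progress widget and enabling crafting at two.
; A tagged player entering the box when stocked can press E to start a timed craft.
; Tick pins the player to the box and drives a progress bar until the delay ends, then the bouquet spawns and the station resets.
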(event OnComponentBeginOverlap(Box)
  (params (OverlappedComponent :type Primitive%20Component%20Object%20Reference) (OtherActor :type Actor%20Object%20Reference) (OtherComp :type Primitive%20Component%20Object%20Reference) (OtherBodyIndex :type Integer) (bFromSweep :type Boolean) (SweepResult :type Hit%20Result%20Structure%20%28by%20ref%29))
  ;[1 1 1] Detect Player
  (if (and (Actor|ActorHasTag OtherActor "Player") (== (Variables|Default|GetFlowerRedNumber) 2))
    (Variables|Default|SetPlayerCanCraft OtherActor)))

(event OnComponentEndOverlap(Box)
  (params (OverlappedComponent :type Primitive%20Component%20Object%20Reference) (OtherActor :type Actor%20Object%20Reference) (OtherComp :type Primitive%20Component%20Object%20Reference) (OtherBodyIndex :type Integer))
  ;[1 1 1] Remove Player From Variable
  (if (Utilities|IsValid (Variables|Default|GetPlayerCanCraft))
    (Variables|Default|SetPlayerCanCraft 0)))

(event Collision|EventActorBeginOverlap
  (params (OtherActor :type Actor%20Object%20Reference))
  (bind _craftingprogress2 (Variables|Default|GetCraftingProgress2))
  ;[1 1 1] Set Bool CanCraft
  (if (and (Actor|ActorHasTag OtherActor "Ingredient") (< (Variables|Default|GetFlowerRedNumber) 2))
    (Actor|DestroyActor OtherActor)
    (bind _result (Math|Integer|IncrementInt (Variables|Default|GetFlowerRedNumber))
      (:%20%20
        (Variables|Default|SetFlowerRedNumber _result)
        (Rendering|SetVisibility _craftingprogress2 true false)
        (bind _asw_progression_circle (Utilities|Casting|CastToW_ProgressionCircle (UserInterface|GetUserWidgetObject _craftingprogress2)))
        (Variables|/Game/SandboxK/UI/W_ProgressionCircle.W_ProgressionCircle_C|SetCraftingProgress _asw_progression_circle (+ (Variables|/Game/SandboxK/UI/W_ProgressionCircle.W_ProgressionCircle_C|GetCraftingProgress _asw_progression_circle) 0.5))
        (if (== (Variables|Default|GetFlowerRedNumber) 2)
          (Variables|Default|SetCanCraft true)
          (else
            (Variables|Default|SetCanCraft false)))))))

(event EventTick
  (params (DeltaSeconds :type Float%20%28single-precision%29))
  (bind _box (Variables|Default|GetBox))
  (bind _craftingprogress (Variables|Default|GetCraftingProgress))
  (bind _returnvalue (Transformation|GetWorldTransform _box))
  (bind (_location _rotation) (Math|Transform|BreakTransform _returnvalue))
  (bind (_roll _pitch _yaw) (Math|Rotator|BreakRotator _rotation))
  ;[1 1 1] Comment
  (if (Variables|Default|GetCrafting)
    (Transformation|SetActorLocationAndRotation (Variables|Default|GetPlayerCanCraft) _location (Math|Rotator|MakeRotator _roll _pitch (- _yaw 1.8e+02)))
    (Rendering|SetVisibility (Variables|Default|GetCraftingProgress2) false false)
    (Rendering|SetVisibility _craftingprogress true false)
    (bind _asw_progression_bar (Utilities|Casting|CastToW_ProgressionBar (UserInterface|GetUserWidgetObject _craftingprogress)))
    (bind _output_get (Variables|Default|SetElapsedTime (+ (Variables|Default|GetElapsedTime) (Utilities|Time|GetWorldDeltaSeconds))))
    (Variables|/Game/SandboxK/UI/W_ProgressionBar.W_ProgressionBar_C|SetCrafting%25 _asw_progression_bar (Math|Float|Clamp(Float) (/ _output_get (Variables|Default|GetCraftingTime))))))

(event Input|KeyboardEvents|E
  (params (Key :type Key%20Structure :default "None"))
  (bind _spawn_point (Variables|Default|GetSpawn%20Point))
  (bind _returnvalue (Transformation|GetWorldLocation _spawn_point))
  (bind (_x _y _z) (Math|Vector|BreakVector _returnvalue))
  ;[1 1 1] Spawn Crafted Item
  (:Pressed
    (if (and (Variables|Default|GetCanCraft) (Utilities|IsValid (Variables|Default|GetPlayerCanCraft)))
      (Variables|Default|SetCrafting true)
      (Utilities|FlowControl|Delay (Variables|Default|GetCraftingTime))
      (Game|SpawnActorfromClass "/Game/SandboxK/Blueprints/BP_Bouquet.BP_Bouquet_C" (Math|Conversions|ToTransform(Vector) (Math|Vector|MakeVector _x _y (+ _z 5e+01))) "Undefined" "MultiplyWithRoot" 0 0)
      (Variables|Default|SetFlowerRedNumber 0)
      (Variables|Default|SetCrafting false)
      (Rendering|SetVisibility (Variables|Default|GetCraftingProgress) false false)
      (Variables|Default|SetElapsedTime 0.0)
      (Variables|/Game/SandboxK/UI/W_ProgressionCircle.W_ProgressionCircle_C|SetCraftingProgress (stale Collision|EventActorBeginOverlap _asw_progression_circle) 0.0))))

(fn ConstructionScript)