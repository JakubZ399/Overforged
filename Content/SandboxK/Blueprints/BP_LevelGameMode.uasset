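; Level game mode that runs a timed round and decides between next level and game over.
; BeginPlay adds a second player if the game instance specifies two, shows the level UI and starts a looping one-second timer.
; The Timer function counts down minutes and seconds, raising the TimerLoop flag at zero.
; Tick polls that flag, then clears the timer, compares Score to PointsToWin, swaps in the result widget and pauses with cursor shown.
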(event EventBeginPlay
  ;[1 1 1] Add Player
  (bind _asmain_game_instance (Utilities|Casting|CastToMainGameInstance (Game|GetGameInstance)))
  (if (== (Variables|/Game/SandboxK/MainGameInstance.MainGameInstance_C|GetNumberOfPlayer _asmain_game_instance) 2)
    (Class|GameplayStatics|CreatePlayer -1))
  (bind _returnvalue (UserInterface|CreateWidget "/Game/SandboxK/UI/W_LevelUI.W_LevelUI_C"))
  (bind _output_get (Variables|Default|SetCurrentWidget _returnvalue))
  (UserInterface|Viewport|AddtoViewport _output_get 0)
  (Variables|Default|SetLevelUI _returnvalue)
  (bind _returnvalue_2 (Utilities|Time|SetTimerbyFunctionName 0 "Timer" 1.0 true)))

(event EventTick
  (params (DeltaSeconds :type Float%20%28single-precision%29))
  (if (Variables|Default|GetTimerLoop)
    (Utilities|Time|ClearandInvalidateTimerbyHandle (stale EventBeginPlay _returnvalue_2))
    (Widget|RemovefromParent (Variables|Default|GetCurrentWidget))
    (if (>= (Variables|Default|GetScore) (Variables|Default|GetPoints%20To%20Win))
      ;[0.125 0.125 0.125] Set NextLevel Widget
      (bind _returnvalue (UserInterface|CreateWidget "/Game/SandboxK/UI/W_NextLevel.W_NextLevel_C"))
      (bind _output_get (Variables|Default|SetCurrentWidget _returnvalue))
      (UserInterface|Viewport|AddtoViewport _output_get 0)
      (else
        ;[0.125 0.125 0.125] Set GameOver Widget
        (bind _returnvalue_2 (UserInterface|CreateWidget "/Game/SandboxK/UI/W_GameOver.W_GameOver_C"))
        (bind _output_get_2 (Variables|Default|SetCurrentWidget _returnvalue_2))
        (UserInterface|Viewport|AddtoViewport _output_get_2 0)))
    (Variables|/Script/Engine.PlayerController|SetbShowMouseCursor (Game|GetPlayerController 0) true)
    (Game|SetGamePaused true)))

(fn ConstructionScript)

(fn Timer
  (if (and (> (Variables|Default|GetSeconds) 0) (>= (Variables|Default|GetMinutes) 0))
    (bind _result (Math|Integer|DecrementInt (Variables|Default|GetSeconds))
      (:%20%20
        (Variables|Default|SetSeconds _result)))
    (elif (<= (Variables|Default|GetMinutes) 0)
      (Variables|Default|SetMinutes 0)
      (Variables|Default|SetSeconds 0)
      (Variables|Default|SetTimerLoop true)
      (else
        (Variables|Default|SetSeconds 59)
        (bind _result_2 (Math|Integer|DecrementInt (Variables|Default|GetMinutes))
          (:%20%20
            (Variables|Default|SetMinutes _result_2)))))))