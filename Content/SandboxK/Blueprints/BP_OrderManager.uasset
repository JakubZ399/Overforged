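; Order manager actor that feeds randomly chosen recipe orders from a data table to the level UI.
; On BeginPlay it registers with BP_LevelGameMode, adds a first order and starts a looping timer with a once-randomized interval, gated by the UI's active-order limit.
; OrderSetup appends to ActiveOrder and caches the latest recipe, image and name for getters.
; RemoveOrderFromArray ignores its ID and always removes index 0.
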(event Custom|AddOrder
  (bind _maxactiveorders (Variables|Default|GetMaxActiveOrders))
  (bind _leveluiref (Variables|Default|GetLevelUIRef))
  ;[1 1 1] Event AddOrder
  ;;[1 1 1] Check Max Active Order
  (bind _returnvalue (Default|CheckMaxActiveOrders _leveluiref _maxactiveorders)) ; Check Max Active Order
  (if (not _returnvalue)
    ;;[1 1 1] Setup Order & Send It To UI (W_LevelUI)
    (bind (_ordertime _indexinactiveorderarray) (CallFunction|OrderSetup)) ; Order Setup
    (Default|AddOrdertoUI _leveluiref _ordertime _maxactiveorders self _indexinactiveorderarray) ; Add Order to UI
  ))

(event Custom|AddFirstOrder
  ;[1 1 1] Event AddOrder
  ;;[1 1 1] Setup Order & Send It To UI (W_LevelUI)
  (bind (_ordertime _indexinactiveorderarray) (CallFunction|OrderSetup)) ; Order Setup
  (Default|AddOrdertoUI (Variables|Default|GetLevelUIRef) _ordertime (Variables|Default|GetMaxActiveOrders) self _indexinactiveorderarray) ; Add Order to UI
)

(event EventBeginPlay
  ;[1 1 1] Setup LevelUI Ref
  (bind _outrownames (DataTable|GetDataTableRowNames (Variables|Default|GetDataTable)))
  (Variables|Default|SetDataTableNameRow _outrownames)
  (Utilities|FlowControl|Delay 0.1)
  (bind _asbp_level_game_mode (Utilities|Casting|CastToBP_LevelGameMode (Game|GetGameMode)))
  (Variables|/Game/SandboxK/Blueprints/BP_LevelGameMode.BP_LevelGameMode_C|SetBP_OrderManagerGM _asbp_level_game_mode self)
  (bind _asw_level_ui (Utilities|Casting|CastToW_LevelUI (Variables|/Game/SandboxK/Blueprints/BP_LevelGameMode.BP_LevelGameMode_C|GetLevelUI _asbp_level_game_mode)))
  (Variables|Default|SetLevelUIRef _asw_level_ui)
  ;[1 1 1] Add Order To UI For Couple Seconds
  (CallFunction|AddFirstOrder)
  (Utilities|Time|SetTimerbyEvent (delegate Custom|AddOrder) (Math|Random|RandomFloatinRange (Variables|Default|GetTimeBetweenOrder_Min) (Variables|Default|GetTimeBetweenOrder_Max)) true))

(fn ConstructionScript)

(fn OrderSetup
  (bind _returnvalue (Utilities|GetDataTableRow (Variables|Default|GetDataTable) (.OutItem (Utilities|Array|Random (Variables|Default|GetDataTableNameRow))))
    (:then
      (Variables|OrderDisplay|SetRecipe (.Recipe (Utilities|Struct|BreakS_Recipe _returnvalue)))
      (Variables|OrderDisplay|SetImage (.Image (Utilities|Struct|BreakS_Recipe _returnvalue)))
      (Variables|OrderDisplay|SetX (.ImageSizeX (Utilities|Struct|BreakS_Recipe _returnvalue)))
      (Variables|OrderDisplay|SetY (.ImageSizeY (Utilities|Struct|BreakS_Recipe _returnvalue)))
      (Variables|Default|SetOrderNameOM (.Name (Utilities|Struct|BreakS_Recipe _returnvalue)))
      (LocalVariables|SetSetupOrder (Utilities|Struct|MakeS_OrderStruck (.ItemCraftingDifficulty (Utilities|Struct|BreakS_Recipe _returnvalue)) (.ItemBP (Utilities|Struct|BreakS_Recipe _returnvalue)) (.Points (Utilities|Struct|BreakS_Recipe _returnvalue)) (.Name (Utilities|Struct|BreakS_Recipe _returnvalue))))
      (bind _returnvalue_2 (Utilities|Array|Add (Variables|Default|GetActiveOrder) (LocalVariables|GetSetupOrder)))
      (return (Variables|Default|GetOrderTime) _returnvalue_2))))

(fn GetOrderInfo
  (return (Variables|OrderDisplay|GetRecipe) (Variables|OrderDisplay|GetImage) (Variables|OrderDisplay|GetX) (Variables|OrderDisplay|GetY)))

(fn GetOrderNameOM
  (return (Variables|Default|GetOrderNameOM)))

(fn RemoveOrderfromArray
  (params (ID :type Integer))
  (Utilities|Array|RemoveIndex (Variables|Default|GetActiveOrder))
  (Development|PrintString "Hello" true true "(R=1.000000,G=0.005026,B=0.000000,A=1.000000)")
  (return))