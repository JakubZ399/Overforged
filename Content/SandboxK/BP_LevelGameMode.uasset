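; Game mode for a level that creates the level UI widget and holds a minutes-and-seconds countdown.
; BeginPlay adds W_LevelUI to the viewport.
; The Timer function decrements Seconds, borrows from Minutes by resetting Seconds to 60, and sets TimerLoop once time runs out.
; Nothing in this graph calls Timer, and Tick checks TimerLoop without acting on it.
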(event EventBeginPlay
  (bind _returnvalue (UserInterface|CreateWidget "/Game/SandboxK/UI/W_LevelUI.W_LevelUI_C"))
  (UserInterface|Viewport|AddtoViewport _returnvalue 0))

(event EventTick
  (params (DeltaSeconds :type Float%20%28single-precision%29))
  (if (Variables|Default|GetTimerLoop)
    _))

(fn ConstructionScript)

(fn Timer
  (if (and (> (Variables|Default|GetSeconds) 0) (>= (Variables|Default|GetMinutes) 0))
    (bind _result (Math|Integer|DecrementInt (Variables|Default|GetSeconds))
      (:%20%20
        (Variables|Default|SetSeconds _result)))
    (elif (<= (Variables|Default|GetMinutes) 0)
      (Variables|Default|SetMinutes 0)
      (Variables|Default|SetSeconds 0)
      (Variables|Default|SetTimerLoop true)
      (else
        (Variables|Default|SetSeconds 60)
        (bind _result_2 (Math|Integer|DecrementInt (Variables|Default|GetMinutes))
          (:%20%20
            (Variables|Default|SetMinutes _result_2)))))))