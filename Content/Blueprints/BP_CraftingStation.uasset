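; Crafting station actor where a player places tagged ingredients into three slots and crafts an item from them.
; An interface call fills the first empty slot, records the ingredient's enum and attaches the actor.
; On the P2 action input, the in-range player triggers an order-sensitive DataTable recipe match, then a timed delay replaces the ingredients with the spawned result.
; Tick pins the player during crafting, and a clear input destroys placed items.
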(event OnComponentBeginOverlap(PlayerCraftingCheck)
  (params (OverlappedComponent :type Primitive%20Component%20Object%20Reference) (OtherActor :type Actor%20Object%20Reference) (OtherComp :type Primitive%20Component%20Object%20Reference) (OtherBodyIndex :type Integer) (bFromSweep :type Boolean) (SweepResult :type Hit%20Result%20Structure%20%28by%20ref%29))
  ;[0.09896 0.09896 0.09896] Detect Player
  (CallFunction|DetectPlayerAdd OtherActor))

(event OnComponentEndOverlap(PlayerCraftingCheck)
  (params (OverlappedComponent :type Primitive%20Component%20Object%20Reference) (OtherActor :type Actor%20Object%20Reference) (OtherComp :type Primitive%20Component%20Object%20Reference) (OtherBodyIndex :type Integer))
  ;[0.09896 0.09896 0.09896] Remove Player From Variable
  (CallFunction|DetectPlayerRemove))

(event Custom|MoveActor
  (bind _item (Variables|Default|GetItem))
  ;[0.09896 0.09896 0.09896] MoveActor
  (Utilities|Array|Add (Variables|Default|GetItemInSlot) _item)
  (Transformation|AttachComponentToComponent _item (Utilities|Array|Get(acopy) (Variables|Default|GetSlots) (Variables|Default|GetIndex)) "None" "KeepWorld" "KeepWorld" "KeepWorld" true)
  (Components|MoveComponentTo (Variables|/Script/Engine.Actor|GetRootComponent (Variables|Default|GetItem)) "0, 0, 0" "0, 0, 0" false false 0.2 false))

(event Input|EnhancedActionEvents|EnhancedInputActionIA_ActionP2
  (params (ActionValue :type Boolean) (ElapsedSeconds :type Float%20%28double-precision%29) (TriggeredSeconds :type Float%20%28double-precision%29) (InputAction :type Input%20Action%20Object%20Reference :default "/Game/Input/Actions/IA_ActionP2.IA_ActionP2"))
  (bind _occupiedslotsenum (Variables|Default|GetOccupiedSlotsEnum))
  (bind _recipetable (Variables|Default|GetRecipeTable))
  ;[0.09896 0.09896 0.09896] Spawn Item System
  (:Started
    (Utilities|IsValid (Variables|Default|GetPlayerWantCraft)
      (:Is%20Valid
        (if (Variables|Default|GetInRange)
          ;;[0.09896 0.09896 0.09896] Check If Slot Are NONE
          (bind _array_element (Utilities|Array|ForEachLoopwithBreak (Variables|Default|GetOccupiedSlotsEnum) :!label _label)
            (:LoopBody
              (if (Utilities|Enum|NotEqual(Enum) _array_element "NewEnumerator5")
                (Variables|Default|SetAllNONE false)
                (goto _label Break)))
            (:Completed
              ;;[0.09896 0.09896 0.09896] Check Recipe Match Witch DataTable
              (if (not (Variables|Default|GetAllNONE))
                (bind _outrownames (DataTable|GetDataTableRowNames _recipetable))
                (bind _array_element_2 (Utilities|Array|ForEachLoopwithBreak _outrownames :!label _label_2)
                  (:LoopBody
                    (bind _returnvalue (Utilities|GetDataTableRow _recipetable _array_element_2)
                      (:then
                        (if (Utilities|Array|Identical (.Recipe (Utilities|Struct|BreakS_Recipe _returnvalue)) (Variables|Default|GetOccupiedSlotsEnum))
                          (Variables|Default|SetRecipeMatches true)
                          (goto _label_2 Break)))))
                  (:Completed
                    (if (Variables|Default|GetRecipeMatches)
                      (Variables|Default|SetCrafting true)
                      (Utilities|FlowControl|Delay (.TimeToCraft (Utilities|Struct|BreakS_Recipe _returnvalue)))
                      (Variables|Default|SetCrafting false)
                      ;;[0.09896 0.09896 0.09896] Spawn Item & Destroy Ingredients
                      (for _array_element_3 (Variables|Default|GetItemInSlot)
                        (Utilities|IsValid _array_element_3
                          (:Is%20Valid
                            (Actor|DestroyActor _array_element_3))))
                      (Game|SpawnActorfromClass (.ItemBP (Utilities|Struct|BreakS_Recipe _returnvalue)) (Math|Conversions|ToTransform(Vector) (Transformation|GetWorldLocation (Variables|Default|GetSpawn%20Point))) "Undefined" "MultiplyWithRoot" 0 0)
                      (Utilities|Array|Clear _occupiedslotsenum)
                      (for _index (range 0 2)
                        (Utilities|Array|Add _occupiedslotsenum "NewEnumerator5")
                        (Variables|Default|SetAllNONE true)))))))))))))

(event Input|EnhancedActionEvents|EnhancedInputActionIA_Clear
  (params (ActionValue :type Boolean) (ElapsedSeconds :type Float%20%28double-precision%29) (TriggeredSeconds :type Float%20%28double-precision%29) (InputAction :type Input%20Action%20Object%20Reference :default "/Game/Input/Actions/IA_Clear.IA_Clear"))
  (bind _occupiedslotsenum (Variables|Default|GetOccupiedSlotsEnum))
  ;[1 0.838 0.3518] Clear For R key
  (:Started
    (if (Variables|Default|GetInRange)
      (for _array_element (Variables|Default|GetItemInSlot)
        (Utilities|IsValid _array_element
          (:Is%20Valid
            (Actor|DestroyActor _array_element)
            (Utilities|Array|Clear _occupiedslotsenum)
            (for _index (range 0 2)
              (Utilities|Array|Add _occupiedslotsenum "NewEnumerator5")
              (Variables|Default|SetAllNONE true))))))))

(event EventTick
  (params (DeltaSeconds :type Float%20%28single-precision%29))
  (bind _playercraftingcheck (Variables|Default|GetPlayerCraftingCheck))
  (bind _returnvalue (Transformation|GetWorldTransform _playercraftingcheck))
  (bind (_location _rotation) (Math|Transform|BreakTransform _returnvalue))
  (bind (_roll _pitch _yaw) (Math|Rotator|BreakRotator _rotation))
  ;[0.09896 0.09896 0.09896] REWORK IT for Progression bar and crafting in place
  (if (Variables|Default|GetCrafting)
    (Transformation|SetActorLocationAndRotation (Variables|Default|GetPlayerWantCraft) _location (Math|Rotator|MakeRotator _roll _pitch (- _yaw 1.8e+02)))))

(fn ConstructionScript
  (Variables|Default|SetSlots (Utilities|Array|MakeArray (Variables|Default|GetPlace%20Item%20Point) (Variables|Default|GetPlace%20Item%20Point1) (Variables|Default|GetPlace%20Item%20Point2))))

(fn DetectPlayerRemove
  (Utilities|IsValid (Variables|Default|GetPlayerWantCraft)
    (:Is%20Valid
      (Variables|Default|SetPlayerWantCraft 0)
      (Variables|Default|SetInRange false))))

(fn DetectPlayerAdd
  (params (InputPin :type Actor%20Object%20Reference))
  (Utilities|IsValid (Variables|Default|GetPlayerWantCraft)
    (:Is%20Not%20Valid
      (if (Actor|ActorHasTag InputPin "Player")
        (Variables|Default|SetPlayerWantCraft InputPin)
        (Variables|Default|SetInRange true)))))

(fn PlaceItemInterface
  (params (ItemToPlace :type Actor%20Object%20Reference))
  (if (Actor|ActorHasTag ItemToPlace "Ingredient")
    (bind (_array_element _array_index) (Utilities|Array|ForEachLoopwithBreak (Variables|Default|GetOccupiedSlotsEnum))
      (:LoopBody
        (if (Utilities|Enum|Equal(Enum) _array_element "NewEnumerator5")
          (Variables|Default|SetIndex _array_index)
          (bind _output_get (Variables|Default|SetItem ItemToPlace))
          (bind _ingredient_enum (Class|BPIItemInterface|GetIngredientEnumValue(Message) _output_get))
          (Utilities|Array|SetArrayElem (Variables|Default|GetOccupiedSlotsEnum) (Variables|Default|GetIndex) _ingredient_enum true)
          (Utilities|Array|AddUnique (Variables|/Script/Engine.Actor|GetTags _output_get) "InCrafting")
          (Transformation|DetachFromActor _output_get "KeepWorld" "KeepWorld" "KeepWorld")
          (CallFunction|MoveActor)
          (return true))))))