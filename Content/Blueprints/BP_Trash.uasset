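; BP_Trash is a trash can actor that accepts an item through the PlaceItemInterface function and destroys it.
; The function stores the item, detaches it, triggers MoveActor and returns true.
; MoveActor attaches the item to ItemLocation, then chains timed MoveComponentTo moves to open the lid, slide the item into the bin, destroy it and close the lid.
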(event Custom|MoveActor
  (bind _itemtodelete (Variables|Default|GetItemToDelete))
  (Transformation|AttachComponentToComponent _itemtodelete (Variables|Default|GetItemLocation) "None" "KeepWorld" "KeepWorld" "KeepWorld" true)
  ;[1 1 1] Open Box_Lid
  (Components|MoveComponentTo (Variables|Default|GetTrash_Can_Box_lid_001) "0.000000,50.000000,180.000000" "0, 0, 0" false false 0.3 false)
  ;[1 1 1] Move Item To Trash
  (Components|MoveComponentTo (Variables|/Script/Engine.Actor|GetRootComponent _itemtodelete) "0, 0, 0" "0, 0, 0" false false 0.3 false)
  (Actor|DestroyActor _itemtodelete)
  ;[1 1 1] Close Box_Lid
  (Components|MoveComponentTo (Variables|Default|GetTrash_Can_Box_lid_001) "0.000000,-50.000000,40.000000" "0, 0, 0" false false 0.5 false))

(event EventBeginPlay)

(event Collision|EventActorBeginOverlap
  (params (OtherActor :type Actor%20Object%20Reference)))

(event EventTick
  (params (DeltaSeconds :type Float%20%28single-precision%29)))

(fn ConstructionScript)

(fn PlaceItemInterface
  (params (ItemToPlace :type Actor%20Object%20Reference))
  (bind _output_get (Variables|Default|SetItemToDelete ItemToPlace))
  (Transformation|DetachFromActor _output_get "KeepWorld" "KeepWorld" "KeepWorld")
  (CallFunction|MoveActor)
  (return true))