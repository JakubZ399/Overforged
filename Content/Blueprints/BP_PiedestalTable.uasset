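; Pedestal table actor that receives one item at a time through a PlaceItemInterface function.
; The function accepts an item only if the ItemPlace component has no children, then detaches it from its parent, calls MoveActor and returns true.
; The MoveActor event attaches the item to ItemPlace keeping world transform, then runs MoveComponentTo on its root, keeping that latent move outside the function.
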(event Custom|MoveActor
  (bind _itemtoplace (Variables|Default|GetItemToPlace))
  (Transformation|AttachComponentToComponent _itemtoplace (Variables|Default|GetItemPlace) "None" "KeepWorld" "KeepWorld" "KeepWorld" true)
  (Components|MoveComponentTo (Variables|/Script/Engine.Actor|GetRootComponent _itemtoplace) "0, 0, 0" "0, 0, 0" false false 0.2 false))

(fn ConstructionScript)

(fn PlaceItemInterface
  (params (ItemToPlace :type Actor%20Object%20Reference))
  (if (Utilities|Array|IsEmpty (Components|GetChildrenComponents (Variables|Default|GetItemPlace) false))
    (bind _output_get (Variables|Default|SetItemToPlace ItemToPlace))
    (Transformation|DetachFromActor _output_get "KeepWorld" "KeepWorld" "KeepWorld")
    (CallFunction|MoveActor)
    (return true)))