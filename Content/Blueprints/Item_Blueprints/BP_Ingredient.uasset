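; BP_Ingredient is an item actor representing an ingredient, with its type chosen by an enum.
; The construction script adds the "Ingredient" tag, finds the data table row named after the enum and applies its mesh, image and image size.
; BeginPlay runs the parent logic, then sets up the display image.
; Getters expose the enum and return zero for crafted points and craft time.
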(event EventBeginPlay
  (|CallParentFunction)
  (CallFunction|SetupDisplayImage))

(event Collision|EventActorBeginOverlap
  (params (OtherActor :type Actor%20Object%20Reference)))

(event EventTick
  (params (DeltaSeconds :type Float%20%28single-precision%29)))

(fn ConstructionScript
  (bind _ingredientdatatable (Variables|Default|GetIngredientDataTable))
  (|CallParentFunction)
  ;[0.09306 0.09306 0.09306] Tag Setup
  (Utilities|Array|AddUnique (Variables|Default|GetTags) "Ingredient")
  (bind _outrownames (DataTable|GetDataTableRowNames _ingredientdatatable))
  (for _array_element _outrownames
    (if (== _array_element (Utilities|String|StringToName (Utilities|String|EnumtoString (Variables|Default|GetEnum))))
      (bind _returnvalue (Utilities|GetDataTableRow _ingredientdatatable _array_element)
        (:then
          (bind _output_get (Variables|Default|SetMainMesh (.Mesh (Utilities|Struct|BreakS_Ingredient _returnvalue))))
          (Variables|Default|SetItemImage (.Image (Utilities|Struct|BreakS_Ingredient _returnvalue)))
          (Variables|Default|SetDesired%20Size%20X (.ImageSizeX (Utilities|Struct|BreakS_Ingredient _returnvalue)))
          (Variables|Default|SetDesired%20Size%20Y (.ImageSizeY (Utilities|Struct|BreakS_Ingredient _returnvalue)))
          (CallFunction|MeshtoRootSetup _output_get))))))

(fn GetCraftedPoints
  (return 0))

(fn GetIngredientEnumValue
  (return (Variables|Default|GetEnum)))

(fn GetTimetoCraftCrafted
  (return 0.0))