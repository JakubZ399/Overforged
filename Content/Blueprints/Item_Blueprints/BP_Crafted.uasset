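; BP_Crafted is a crafted item that rots once its timer runs out.
; Construction tags it "Crafted" and copies the RecipeDataTable row matching its ID into its name, points, craft time, difficulty, mesh and image, with image X/Y sizes swapped.
; BeginPlay sets up the display image and starts the timer, which replaces the tags with "Rotten" and updates the W_Flower widget and name.
; Getters expose points, craft time and a fixed ingredient enum.
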(event Custom|ChangeToRotten
  ;[1 1 1] Comment
  (Variables|Default|SetTags (Utilities|Array|MakeArray "Rotten"))
  (Development|PrintString "ROTTEN")
  (bind _asw_flower (Utilities|Casting|CastToW_Flower (UserInterface|GetWidget (Variables|Default|GetImage2D))))
  ;;[1 1 1] Setup Display Image Over Object
  (Utilities|FlowControl|Sequence
    (:then_0
      (Variables|/Game/UI/LevelUI/W_Flower.W_Flower_C|SetPopUpSlateBrush _asw_flower (Variables|Default|GetRottenFlower)))
    (:then_1
      (Variables|/Game/UI/LevelUI/W_Flower.W_Flower_C|SetImage%20Size%20X _asw_flower 4e+01))
    (:then_2
      (Variables|/Game/UI/LevelUI/W_Flower.W_Flower_C|SetImage%20Size%20Y _asw_flower 6e+01))
    (:then_3
      (Variables|Default|SetName "Rotten"))))

(event EventBeginPlay
  (|CallParentFunction)
  (CallFunction|SetupDisplayImage)
  ;[1 1 1] Comment
  (Utilities|Time|SetTimerbyEvent (delegate Custom|ChangeToRotten) (Variables|Default|GetTimeToRotten)))

(event Collision|EventActorBeginOverlap
  (params (OtherActor :type Actor%20Object%20Reference)))

(event EventTick
  (params (DeltaSeconds :type Float%20%28single-precision%29)))

(fn ConstructionScript
  (bind _recipe_datatable (Variables|Default|GetRecipe%20DataTable))
  (|CallParentFunction)
  ;[0.09306 0.09306 0.09306] Tag Setup
  (Utilities|Array|AddUnique (Variables|Default|GetTags) "Crafted")
  (bind _outrownames (DataTable|GetDataTableRowNames _recipe_datatable))
  (for _array_element _outrownames
    (if (== _array_element (Variables|Default|GetID))
      (bind _returnvalue (Utilities|GetDataTableRow _recipe_datatable _array_element)
        (:then
          (Variables|Default|SetName (.Name (Utilities|Struct|BreakS_Recipe _returnvalue)))
          (Variables|Default|SetPoints (.Points (Utilities|Struct|BreakS_Recipe _returnvalue)))
          (Variables|Default|SetTimeToCraft (.TimeToCraft (Utilities|Struct|BreakS_Recipe _returnvalue)))
          (bind _output_get (Variables|Default|SetMainMesh (.Mesh (Utilities|Struct|BreakS_Recipe _returnvalue))))
          (Variables|Default|SetItemImage (.Image (Utilities|Struct|BreakS_Recipe _returnvalue)))
          (Variables|Default|SetDesired%20Size%20Y (.ImageSizeX (Utilities|Struct|BreakS_Recipe _returnvalue)))
          (Variables|Default|SetDesired%20Size%20X (.ImageSizeY (Utilities|Struct|BreakS_Recipe _returnvalue)))
          (Variables|Default|SetDifficulty (.ItemCraftingDifficulty (Utilities|Struct|BreakS_Recipe _returnvalue)))
          (CallFunction|MeshtoRootSetup _output_get))))))

(fn GetCraftedPoints
  (return (Variables|Default|GetPoints)))

(fn GetIngredientEnumValue
  (return "NewEnumerator0"))

(fn GetTimetoCraftCrafted
  (return (Variables|Default|GetTimeToCraft)))