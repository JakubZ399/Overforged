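; Player interaction scene component for grabbing items, placing them on tables and retrieving them from storage boxes.
; Each tick a forward line trace highlights the hit actor with an overlay material and moves any held item to the trace end, disabling its physics.
; The action input sphere-traces to grab or flags a release, then calls the table interface or storage box, with HaveItem and WannaRelase tracking hold state.
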(event Custom|Interaction
  (bind _currenthitactor (Variables|Default|GetCurrentHitActor))
  ;[0.09896 0.09896 0.09896] Interaction
  (bind _bool (CallFunction|Find,Take&Relase (Variables|Default|GetHaveItem)))
  (if _bool
    (Utilities|IsValid _currenthitactor
      (:Is%20Valid
        (bind _returnvalue (Interaction|InterfaceandItemCheck _currenthitactor))
        (if _returnvalue
          (Interaction|PlaceonTable)
          (else
            (Interaction|RetrieveStorageItem)))))))

(event Input|EnhancedActionEvents|EnhancedInputActionIA_ActionP1
  (params (ActionValue :type Boolean) (ElapsedSeconds :type Float%20%28double-precision%29) (TriggeredSeconds :type Float%20%28double-precision%29) (InputAction :type Input%20Action%20Object%20Reference :default "/Game/Input/Actions/IA_ActionP1.IA_ActionP1"))
  ;[0.09896 0.09896 0.09896] Interaction Key
  (:Started
    (CallFunction|Interaction)))

(event EventTick
  (params (DeltaSeconds :type Float%20%28single-precision%29))
  ;[0.09896 0.09896 0.09896] Tick
  (CallFunction|CalculatePositionVector)
  ;;[0.09896 0.09896 0.09896] HighLight
  (bind (_outhit _returnvalue) (Collision|LineTraceByChannel (Variables|Default|GetStart) (Variables|Default|GetEnd) "TraceTypeQuery4" false 0 "None"))
  (bind _output_get (Variables|Default|SetHasDetectEnv _returnvalue))
  (CallFunction|ChangeHighlight _output_get (.HitActor (Collision|BreakHitResult _outhit)))
  (Utilities|IsValid (Variables|Default|GetCurrentHitActor)
    (:Is%20Valid
      (if (> (Math|Vector|Distance(Vector) (Transformation|GetActorLocation (Variables|Default|GetCurrentHitActor)) (Transformation|GetWorldLocation)) (+ (Variables|Default|GetGrabbingDistance) 1e+02))
        (Variables|Default|SetCurrentHitActor 0)))
    (:Is%20Not%20Valid
      _))
  ;[0.09896 0.09896 0.09896] Grab Item
  (bind _returnvalue_2 (GrabItem|ToggleItemHoldBool))
  (if _returnvalue_2
    (GrabItem|MoveGrabbedActor/Change)
    (else
      (GrabItem|RelaseGrabbedActor/Change))))

(event EventBeginPlay
  ;[0.09896 0.09896 0.09896] BeginPlay
  (CallFunction|HandSetup))

(fn CalculatePositionVector
  (bind _output_get (Variables|Default|SetStart (Transformation|GetWorldLocation)))
  (Variables|Default|SetEnd (+ _output_get (* (Math|Vector|GetForwardVector) (Variables|Default|GetGrabbingDistance))))
  (return))

(fn ChangeHighlight
  (params (Condition :type Boolean) (CurrentHitActor :type Actor%20Object%20Reference))
  (if Condition ; Detect Hit
    ;[1 1 1] Set HighLight Material
    (bind _output_get (Variables|Default|SetCurrentHitActor CurrentHitActor))
    (bind _array_element (Utilities|Array|ForEachLoopwithBreak (Actor|GetComponentsByClass _output_get "/Script/Engine.MeshComponent"))
      (:LoopBody
        (Rendering|Material|SetOverlayMaterial _array_element "/Game/Materials/M_HighLightPROTOTYPE.M_HighLightPROTOTYPE" :!class /Script/Engine.MeshComponent))
      (:Completed
        ;[1 1 1] Set LastHitActor Material To NONE
        (if (and (!= _output_get (Variables|Default|GetLastHitActor)) (!= (Variables|Default|GetLastHitActor) 0))
          (bind _array_element_2 (Utilities|Array|ForEachLoopwithBreak (Actor|GetComponentsByClass (Variables|Default|GetLastHitActor) "/Script/Engine.MeshComponent") :!label _label)
            (:LoopBody
              (Rendering|Material|SetOverlayMaterial _array_element_2 0 :!class /Script/Engine.MeshComponent))
            (:Completed
              (Variables|Default|SetLastHitActor (Variables|Default|GetCurrentHitActor) :!label _label_2)
              (return)))
          (else
            (goto _label_2)))))
    (else
      ;[1 0 0.03182] If You Change Look You Change Overlay to NONE
      (if (!= (Variables|Default|GetLastHitActor) 0)
        (goto _label)))))

(fn Find,Take&Relase
  (params (Condition :type Boolean))
  (bind _start (Variables|Default|GetStart))
  (bind _end (Variables|Default|GetEnd))
  (bind (_x _y _z) (Math|Vector|BreakVector _start))
  (bind (_x_2 _y_2 _z_2) (Math|Vector|BreakVector _end))
  (if Condition
    (if (Utilities|DoesObjectImplementInterface (Variables|Default|GetCurrentHitActor) "/Game/Blueprints/BPI_TableInteraction.BPI_TableInteraction_C")
      (return "true")
      (else
        (Variables|Default|SetWannaRelase true)
        (return "false")))
    (else
      (bind (_outhit _returnvalue) (Collision|SphereTraceByChannel (Math|Vector|MakeVector _x _y (+ _z 5e+01)) (Math|Vector|MakeVector _x_2 _y_2 (+ _z_2 5e+01)) 5e+01 "TraceTypeQuery3" false 0 "None"))
      (if _returnvalue
        (if (not (Actor|ActorHasTag (.HitActor (Collision|BreakHitResult _outhit)) "InCrafting"))
          (Variables|Default|SetHaveItem true)
          (Variables|Default|SetGrabbedActor (.HitActor (Collision|BreakHitResult _outhit)))
          (Variables|Default|SetGrabbedItem (.HitComponent (Collision|BreakHitResult _outhit)))
          (return "false"))
        (else
          (return "true"))))))

(fn HandSetup
  (Variables|Default|SetHand (Components|GetChildComponent self 0)))

(fn RetrieveStorageItem
  (bind _currenthitactor (Variables|Default|GetCurrentHitActor))
  ;[1 1 1] Take Item From BP_StorageBox
  (if (and (Variables|Default|GetHasDetectEnv) (and (Actor|ActorHasTag _currenthitactor "StorageBox") (not (Variables|Default|GetHaveItem))))
    (Class|BPIStorageInteraction|AddItem(Message) _currenthitactor)))

(fn PlaceonTable
  (bind _grabbedactor (Variables|Default|GetGrabbedActor))
  (bind _currenthitactor (Variables|Default|GetCurrentHitActor))
  ;[1 1 1] Place Item On Table Object
  (Utilities|IsValid _grabbedactor
    (:Is%20Valid
      (Utilities|IsValid _currenthitactor
        (:Is%20Valid
          (bind _newparam (Class|BPITableInteraction|PlaceItemInterface(Message) _currenthitactor _grabbedactor))
          (if _newparam
            (Variables|Default|SetWannaRelase true)
            (Variables|Default|SetHaveItem false)))))))

(fn InterfaceandItemCheck
  (params (CurrentHitActor :type Object%20Object%20Reference))
  (return (and (Utilities|DoesObjectImplementInterface CurrentHitActor "/Game/Blueprints/BPI_TableInteraction.BPI_TableInteraction_C") (Variables|Default|GetHaveItem))))

(fn MoveGrabbedActor/Change
  (bind _end (Variables|Default|GetEnd))
  (bind (_x _y _z) (Math|Vector|BreakVector _end))
  (Transformation|SetActorLocationAndRotation (Variables|Default|GetGrabbedActor) (Math|Vector|MakeVector _x _y (+ _z (Variables|Default|GetGrabbingHeight))))
  (if (Utilities|IsValid (Variables|Default|GetGrabbedItem))
    (Physics|SetSimulatePhysics (Variables|Default|GetGrabbedItem) false)))

(fn RelaseGrabbedActor/Change
  (if (Variables|Default|GetHaveItem)
    (Variables|Default|SetGrabbedActor 0)
    (Variables|Default|SetGrabbedItem 0)
    (Variables|Default|SetHaveItem false)
    (Variables|Default|SetWannaRelase false)))

(fn ToggleItemHoldBool
  (Utilities|IsValid (Variables|Default|GetGrabbedActor)
    (:Is%20Valid
      (bind _output_get (Variables|Default|SetHaveItem true))
      (return (and _output_get (not (Variables|Default|GetWannaRelase)))))
    (:Is%20Not%20Valid
      (bind _output_get_2 (Variables|Default|SetHaveItem false))
      (return _output_get_2))))